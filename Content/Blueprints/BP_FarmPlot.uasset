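; BP_FarmPlot is a farm plot actor that players look at and interact with to advance its soil state and plant carrot seeds.
; InteractWith steps a soil enum and swaps the cube's material, consuming a CarrotSeed from the interacter's inventory component for the planting step.
; LookAt shows a tooltip widget until planting, and StopLookAt removes it.
; OpenMe only returns true; its dual-inventory widget code is disconnected.
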(event Input|EnhancedActionEvents|EnhancedInputActionIA_Open
  (params (ActionValue :type Boolean) (ElapsedSeconds :type Float%20%28double-precision%29) (TriggeredSeconds :type Float%20%28double-precision%29) (InputAction :type Input%20Action%20Object%20Reference :default "/Game/TopDown/Input/Actions/IA_Open.IA_Open")))

(event EventBeginPlay)

(event Collision|EventActorBeginOverlap
  (params (OtherActor :type Actor%20Object%20Reference)))

(event EventTick
  (params (DeltaSeconds :type Float%20%28single-precision%29)))

(fn ConstructionScript)

(fn Interactwith
  (params (Interacter :type BP%20Top%20Down%20Character%20Object%20Reference))
  (if (< (Variables|Default|GetSoil) (Math|Conversions|ToInteger(Byte) (Utilities|Enum|LiteralenumENUM_SoilState "NewEnumerator1")))
    (bind _output_get (Variables|Default|SetSoil (Utilities|Enum|ByteToEnumENUM_SoilState (+ (Variables|Default|GetSoil) 1))))
    (Rendering|Material|SetMaterial (Variables|Default|GetCube) 0 "/Game/Imports/3D/brownDark.brownDark")
    (Development|PrintString (Utilities|String|EnumtoString _output_get))
    (return false)
    (else
      (bind _keys (Utilities|Map|Keys (Variables|/Game/Blueprints/BPC_InventoryComponent.BPC_InventoryComponent_C|GetInventoryContent (Variables|/Game/TopDown/Blueprints/BP_TopDownCharacter.BP_TopDownCharacter_C|GetBPC_InventoryComponent Interacter))))
      (if (Utilities|Array|ContainsItem _keys "CarrotSeed")
        (if (< (Variables|Default|GetSoil) (Math|Conversions|ToInteger(Byte) (Utilities|Enum|LiteralenumENUM_SoilState "NewEnumerator2")))
          (bind _output_get_2 (Variables|Default|SetSoil (Utilities|Enum|ByteToEnumENUM_SoilState (+ (Variables|Default|GetSoil) 1))))
          (Rendering|Material|SetMaterial (Variables|Default|GetCube) 0 "/Game/StarterContent/Materials/M_Ground_Gravel.M_Ground_Gravel")
          (Default|RemovefromInventory (Variables|/Game/TopDown/Blueprints/BP_TopDownCharacter.BP_TopDownCharacter_C|GetBPC_InventoryComponent Interacter) "CarrotSeed" 1)
          (Development|PrintString (Utilities|String|EnumtoString _output_get_2)))
        (else
          (Development|PrintString "You need seeds mother fucker"))))))

(fn Lookat
  (params (Observer :type BP%20Top%20Down%20Character%20Object%20Reference))
  (if (Utilities|Enum|NotEqual(Enum) (Variables|Default|GetSoil) "NewEnumerator2")
    (bind _returnvalue (UserInterface|CreateWidget "/Game/Blueprints/UMG_PlayerTooltip.UMG_PlayerTooltip_C"))
    (bind _output_get (Variables|Default|SetPlayerTooltip _returnvalue))
    (UserInterface|Viewport|AddtoViewport _output_get 0)
    (return (Utilities|Text|ToText(String) (Variables|Default|GetName)) "None")))

(fn OpenMe
  (params (Interacter :type BP%20Top%20Down%20Character%20Object%20Reference))
  (return true))

(fn StopLookat
  (params (Observer :type BP%20Top%20Down%20Character%20Object%20Reference))
  (bind _playertooltip (Variables|Default|GetPlayerTooltip)
    (:then
      (Widget|RemovefromParent _playertooltip)
      (Variables|Default|SetPlayerTooltip 0)
      (return ""))
    (:else)))