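; BP_Items is a pickup item actor configured by a data table row handle.
; On BeginPlay it looks up the row to set the cube component's mesh and scale, then writes each mesh material to slot 0, so the last one wins.
; InteractWith adds one of the item to the interacter's inventory component and destroys the actor.
; LookAt returns the row name as the message, while OpenMe always returns false.
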(event EventBeginPlay
  (bind _itemdata (Variables|Default|GetItemData))
  (bind _cube (Variables|Default|GetCube))
  (bind _returnvalue (Utilities|GetDataTableRow (.datatable _itemdata) (.rowname _itemdata))
    (:then
      (Components|StaticMesh|SetStaticMesh _cube (.3DMesh (Utilities|Struct|BreakItemStruct _returnvalue)))
      (Transformation|SetWorldScale3D _cube (* "0.250000,0.250000,0.250000" (.MeshScale (Utilities|Struct|BreakItemStruct _returnvalue))))
      (for _array_element (Variables|/Script/Engine.StaticMesh|GetStaticMaterials (.3DMesh (Utilities|Struct|BreakItemStruct _returnvalue)))
        (Rendering|Material|SetMaterial _cube 0 (.MaterialInterface (Utilities|Struct|BreakStaticMaterial _array_element)))))))

(fn ConstructionScript)

(fn Interactwith
  (params (Interacter :type BP%20Top%20Down%20Character%20Object%20Reference))
  (Default|AddtoInventory (Variables|/Game/TopDown/Blueprints/BP_TopDownCharacter.BP_TopDownCharacter_C|GetBPC_InventoryComponent Interacter) (.rowname (Variables|Default|GetItemData)) 1)
  (Actor|DestroyActor)
  (return true))

(fn Lookat
  (params (Observer :type BP%20Top%20Down%20Character%20Object%20Reference))
  (return (Utilities|Text|ToText(Name) (.RowName (Utilities|Struct|BreakDataTableRowHandle (Variables|Default|GetItemData)))) "None"))

(fn OpenMe
  (params (Interacter :type BP%20Top%20Down%20Character%20Object%20Reference))
  (return false))

(fn StopLookat
  (params (Observer :type BP%20Top%20Down%20Character%20Object%20Reference))
  (return ""))